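; MainGamemode is a game mode Blueprint that runs periodic target spawning and keeps the player's score.
; A looping timer gathers available Target actors into EligableActors, which is never cleared, and calls SpawnTarget on a random pick.
; AddPoints adds points scaled by ScoreMultiplier to Score.
; Tick eases ScoreBuffer toward Score with FInterpTo, giving a smoothed score value.
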(event Custom|Spawn%20Target
  (CallFunction|SpawnTargetFunc))

(event EventBeginPlay
  (Utilities|Time|SetTimerbyEvent (delegate Custom|Spawn%20Target) 1.5 true))

(event EventTick
  (params (DeltaSeconds :type Float%20%28single-precision%29))
  (|InterpScoreBuffer DeltaSeconds))

(fn ConstructionScript)

(fn AddPoints
  (params (Points :type Float%20%28single-precision%29))
  (Variables|Scoring|SetScore (+ (Variables|Scoring|GetScore) (* Points (Variables|Scoring|GetScore%20Multiplier)))))

(fn SpawnTargetFunc
  (bind _eligable_actors (LocalVariables|GetEligable%20Actors))
  (bind _outitem (Utilities|Array|Random _eligable_actors))
  (bind _outactors (Actor|GetAllActorsOfClass "/Game/Main/Blueprints/Targets/Target.Target_C"))
  (bind _array_element (Utilities|Array|ForEachLoopwithBreak _outactors)
    (:LoopBody
      (if (Variables|/Game/Main/Blueprints/Targets/Target.Target_C|GetAvailable _array_element)
        (Utilities|Array|AddUnique (LocalVariables|GetEligable%20Actors) _array_element)))
    (:Completed
      (Utilities|IsValid _outitem
        (:Is%20Valid
          (Default|SpawnTarget _outitem))))))