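; MainPC is a player controller that makes the view drift with a sway that weakens as a Focus value rises.
; Each tick, a curve-driven speed and a turning angle, randomly reversed by a timer, move a smoothed sway rotation added to mouse look.
; Focus eases toward gamepad or key input, driving post-process vignette and a "Pixels" material collection parameter.
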(event Custom|Switch%20Sway%20Turn%20Direction%20Chance%20Event
  (if (Math|Random|RandomBoolwithWeight (Variables|Sway|Turning|GetTurn%20Chance))
    (Variables|Sway|Turning|SetSway%20Direction (not (Variables|Sway|Turning|GetSway%20Direction)))))

(event EventBeginPlay
  (Utilities|Time|SetTimerbyEvent (delegate Custom|Switch%20Sway%20Turn%20Direction%20Chance%20Event) 0.1 true))

(event EventTick
  (params (DeltaSeconds :type Float%20%28single-precision%29))
  (Utilities|FlowControl|Sequence
    (:then_0
      (|SwaySpeedSetting DeltaSeconds))
    (:then_1
      (|SwayandControlRotationSetting DeltaSeconds))
    (:then_2
      (|FocusInterp DeltaSeconds))
    (:then_3
      (|SwayTurning DeltaSeconds))
    (:then_4
      (|FocusVisualEffects))))

(event Input|GamepadEvents|GamepadLeftX
  (params (AxisValue :type Float%20%28single-precision%29))
  (if (Variables|Focus|GetUse%20Gamepad)
    (Variables|Focus|SetRaw%20Focus AxisValue)))

(event Input|KeyboardEvents|Add
  (params (Key :type Key%20Structure :default "None"))
  (:Pressed
    (Variables|Focus|SetRaw%20Focus (Math|Float|Clamp(Float) (+ (Variables|Focus|GetRaw%20Focus) 0.05)))))

(event Input|KeyboardEvents|Subtract
  (params (Key :type Key%20Structure :default "None"))
  (:Pressed
    (Variables|Focus|SetRaw%20Focus (Math|Float|Clamp(Float) (- (Variables|Focus|GetRaw%20Focus) 0.05)))))

(event Input|MouseEvents|Mouse2D
  (params (AxisValue :type Vector :default "0, 0, 0"))
  (Variables|Sway|SetMouse%20Rotation (Math|Rotator|MakeRotator 0.0 (+ (.pitch (Variables|Sway|GetMouse%20Rotation)) (.y AxisValue)) (+ (.yaw (Variables|Sway|GetMouse%20Rotation)) (.x AxisValue)))))

(fn ConstructionScript)