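; MainPawn is a pawn Blueprint that fires darts and produces synthesized audio.
; On BeginPlay it triggers a single timed note on its granular synth.
; Shoot spawns a Dart at the pawn's transform, owned and instigated by the pawn, then plays the gun sound.
; The Focus input is scaled and clamped into an integer FocusLevel parameter on that sound, so the shot audio can vary with focus.
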(event EventBeginPlay
  (Class|GranularSynth|Noteon (Variables|Default|GetGranularSynth) 1e+02 100 1e+01))

(event Collision|EventActorBeginOverlap
  (params (OtherActor :type Actor%20Object%20Reference)))

(event EventTick
  (params (DeltaSeconds :type Float%20%28single-precision%29)))

(fn ConstructionScript)

(fn Shoot
  (params (Focus :type Float%20%28single-precision%29))
  (bind _self self)
  (Utilities|FlowControl|Sequence
    (:then_0
      (Game|SpawnActorfromClass "/Game/Main/Blueprints/Objects/Dart.Dart_C" (Transformation|GetActorTransform) "AlwaysSpawn" _self _self))
    (:then_1
      (Effects|Components|ParticleSystem|SetIntParameter (Variables|Default|GetGun%20Shoot%20Sound) "FocusLevel" (Math|Integer|Clamp(Integer) (Math|Float|Floor (* Focus 4.0)) 0 3))
      (Audio|Components|Audio|Play (Variables|Default|GetGun%20Shoot%20Sound) 0.0))))