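; Player character Blueprint that moves, aims and shoots, with Focused and Aiming states read from Gameplay Ability System tags.
; It starts with a Focused effect; Tick pitches the rotation point, slows walking while aiming and eases Heat toward a focus-dependent baseline.
; Shoot line-traces to hit Targets when focused, otherwise spawns a Dart, with sound varying by MainPC Focus.
; Helpers burst Heat and look up state-transition montages.
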(event EventBeginPlay
  (GameplayEffects|ApplyGameplayEffectToSelf :self (Variables|Default|GetAbilityComponent) :GameplayEffectClass "/Game/Main/Blueprints/Abilities/Effects/FocusedEffect.FocusedEffect_C"))

(event EventTick
  (params (DeltaSeconds :type Float%20%28single-precision%29))
  (Utilities|FlowControl|Sequence
    (:then_0
      (|SetRotation))
    (:then_1
      (|SetMoveSpeed))
    (:then_2
      (|InterpHeat DeltaSeconds))))

(event Input|AxisEvents|InputAxisForward
  (params (AxisValue :type Float%20%28single-precision%29))
  (Class|PawnMovementComponent|AddInputVector (Variables|Character|GetCharacterMovement) (* (Transformation|GetActorForwardVector) AxisValue) false))

(event Input|AxisEvents|InputAxisRight
  (params (AxisValue :type Float%20%28single-precision%29))
  (Class|PawnMovementComponent|AddInputVector (Variables|Character|GetCharacterMovement) (* (Transformation|GetActorRightVector) AxisValue) false))

(fn ConstructionScript)

(fn GetFocus
  (bind _asmain_pc (Utilities|Casting|CastToMainPC (Game|GetPlayerController 0)))
  (return (Variables|/Game/Main/Blueprints/Character/MainPC.MainPC_C|GetFocus _asmain_pc)))

(fn Shoot
  (bind _gun (Variables|Default|GetGun))
  (bind _returnvalue (Transformation|GetSocketLocation _gun "ShootSocket"))
  (Utilities|FlowControl|Sequence
    (:then_0
      (if (CallFunction|IsFocused)
        (bind (_outhit _returnvalue_2) (Collision|LineTraceByChannel _returnvalue (+ (* (Math|Vector|GetForwardVector (Transformation|GetWorldRotation (Variables|Default|GetRotationPoint))) 3e+03) _returnvalue) "TraceTypeQuery1" false 0 "ForDuration"))
        (if _returnvalue_2
          (bind _astarget (Utilities|Casting|CastToTarget (.HitActor (Collision|BreakHitResult _outhit))))
          (Default|Hit _astarget true))
        (else
          (|SpawnDart))))
    (:then_2
      (Effects|Components|ParticleSystem|SetIntParameter (Variables|Default|GetShoot%20Sound) "FocusLevel" (Math|Integer|Clamp(Integer) (Math|Float|Floor (* (CallFunction|GetFocus) 4.0)) 0 3))
      (Audio|Components|Audio|Play (Variables|Default|GetShoot%20Sound) 0.0))))

(fn GetMontageTransition
  (params (Previous :type Focused%20Aiming%20State%20Structure) (Next :type Focused%20Aiming%20State%20Structure))
  (bind (_aiming _focused) (Utilities|Struct|BreakFocusedAimingState Previous))
  (bind (_aiming_2 _focused_2) (Utilities|Struct|BreakFocusedAimingState Next))
  (for _array_element (Variables|Default|GetMontage%20Transitions)
    (if (Math|Boolean|ANDBoolean (Math|Boolean|Equal(Boolean) (.Aiming (Utilities|Struct|BreakFocusedAimingState (.Previous (Utilities|Struct|BreakMontageTransition _array_element)))) _aiming) (Math|Boolean|Equal(Boolean) (.Focused (Utilities|Struct|BreakFocusedAimingState (.Previous (Utilities|Struct|BreakMontageTransition _array_element)))) _focused) (Math|Boolean|Equal(Boolean) (.Aiming (Utilities|Struct|BreakFocusedAimingState (.Next (Utilities|Struct|BreakMontageTransition _array_element)))) _aiming_2) (Math|Boolean|Equal(Boolean) (.Focused (Utilities|Struct|BreakFocusedAimingState (.Next (Utilities|Struct|BreakMontageTransition _array_element)))) _focused_2))
      (return (.Montage (Utilities|Struct|BreakMontageTransition _array_element))))))

(fn IsFocused
  (return (GameplayTags|HasMatchingGameplayTag (Variables|Default|GetAbilityComponent) "(TagName=\"State.Focused\")")))

(fn IsAiming
  (return (GameplayTags|HasMatchingGameplayTag (Variables|Default|GetAbilityComponent) "(TagName=\"State.Aiming\")")))

(fn BurstHeat
  (Variables|Default|SetHeat 1e+02))