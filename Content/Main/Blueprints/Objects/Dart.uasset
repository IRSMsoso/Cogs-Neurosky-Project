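; Dart projectile that launches forward along its local X axis and scores hits on Target actors.
; While flying, Tick aligns it to its velocity with a yaw offset for the mesh.
; The first mesh hit stops movement and calls OnHit, an empty hook here.
; A Target receives the distance from the launch point and the shooter, then the dart is destroyed; on other surfaces it remains.
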(event OnComponentHit(StaticMesh)
  (params (HitComponent :type Primitive%20Component%20Object%20Reference) (OtherActor :type Actor%20Object%20Reference) (OtherComp :type Primitive%20Component%20Object%20Reference) (NormalImpulse :type Vector :default "0, 0, 0") (Hit :type Hit%20Result%20Structure%20%28by%20ref%29))
  (if (Variables|Default|GetFlying)
    (Game|Components|ProjectileMovement|StopSimulating (Variables|Default|GetProjectileMovement) Hit)
    (Variables|Default|SetFlying false)
    (CallFunction|OnHit Hit)
    (bind _astarget (Utilities|Casting|CastToTarget (.HitActor (Collision|BreakHitResult Hit))))
    (Default|Hit _astarget false (Math|Vector|Distance(Vector) (Transformation|GetActorLocation) (Variables|Default|GetInitial%20Location)) 0.0 0 (Variables|Default|GetShooter))
    (Actor|DestroyActor)))

(event EventBeginPlay
  (Game|Components|ProjectileMovement|SetVelocityinLocalSpace (Variables|Default|GetProjectileMovement) "1800.000000,0.000000,0.000000")
  (Variables|Default|SetInitial%20Location (Transformation|GetActorLocation)))

(event Collision|EventActorBeginOverlap
  (params (OtherActor :type Actor%20Object%20Reference)))

(event EventTick
  (params (DeltaSeconds :type Float%20%28single-precision%29))
  (if (Variables|Default|GetFlying)
    (Transformation|SetActorRotation (Math|Rotator|CombineRotators "90.000000, 0, 0" (Math|Conversions|RotationFromXVector (Transformation|GetVelocity))))))

(fn ConstructionScript)

(fn OnHit
  (params (Hit%20Result :type Hit%20Result%20Structure)))