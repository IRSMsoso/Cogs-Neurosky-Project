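; Shootable target scaled by Size that dissolves in when spawned and awards points to the game mode when hit.
; Tick interpolates a dissolve parameter on a dynamic material.
; Normal hits dissolve it out until a cooldown makes it available again, while focused hits permanently shatter a Chaos geometry collection with a strain field.
; Score multiplies focus, distance, heat, streak, quick-shot and inverse-size factors, shown as a popup through the shooter's controller.
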(event EventBeginPlay
  (bind _returnvalue (Rendering|Material|CreateDynamicMaterialInstance (Variables|Default|GetStaticMesh) 0 "/Game/Main/Meshes/Target_Mat_Inst.Target_Mat_Inst" "None" :!class /Script/Engine.PrimitiveComponent))
  (Variables|Default|SetTarget%20Material _returnvalue))

(event Collision|EventActorBeginOverlap
  (params (OtherActor :type Actor%20Object%20Reference)))

(event EventTick
  (params (DeltaSeconds :type Float%20%28single-precision%29))
  (bind _output_get (Variables|Dissolve|SetCurrent%20Dissolve (Math|Interpolation|FInterpTo (Variables|Dissolve|GetCurrent%20Dissolve) (Variables|Dissolve|GetTarget%20Dissolve) DeltaSeconds (Variables|Dissolve|GetDissolve%20Speed))))
  (Rendering|Material|SetScalarParameterValue (Variables|Default|GetTarget%20Material) "Dissolve" _output_get :!class /Script/Engine.MaterialInstanceDynamic))

(fn ConstructionScript
  (bind _size (Variables|Default|GetSize))
  (Transformation|SetActorScale3D (Math|Vector|MakeVector _size _size _size)))

(fn SpawnTarget
  (Variables|Default|SetAvailable false)
  (Variables|Default|SetTargetable true)
  (Collision|SetCollisionEnabled (Variables|Default|GetStaticMesh) "QueryAndPhysics")
  (Variables|Dissolve|SetTarget%20Dissolve 1.0)
  (Variables|Dissolve|SetDissolve%20Speed 7.0))

(fn Hit
  (params (Focused :type Boolean) (Distance :type Float%20%28single-precision%29) (Heat :type Float%20%28single-precision%29) (Hits%20in%20a%20row :type Integer) (Hit%20By :type BP%20Main%20Character%20Object%20Reference))
  (bind _target_collection (Variables|Default|GetTarget_Collection))
  (if (and (Variables|Default|GetTargetable) (not (Variables|Default|GetDestroyed)))
    (Utilities|FlowControl|Sequence
      (:then_0
        (if Focused
          (Development|SetHiddeninGame (Variables|Default|GetStaticMesh) true false)
          (Development|SetHiddeninGame _target_collection false false)
          (Physics|SetSimulatePhysics _target_collection true)
          (Class|GeometryCollectionComponent|ApplyPhysicsField (Variables|Default|GetTarget_Collection) true "Chaos_ExternalClusterStrain" 0 (Field|SetRadialFalloff (Variables|Default|GetRadialFalloff) 1e+06 0.0 1.0 0.0 (* 1.2e+02 (Variables|Default|GetSize)) (Transformation|GetWorldLocation (Variables|Default|GetStaticMesh)) "Field_FallOff_None"))
          (Variables|Default|SetDestroyed true)
          (Collision|SetCollisionEnabled (Variables|Default|GetStaticMesh) "NoCollision")
          (Utilities|Time|SetTimerbyFunctionName 0 "Hide Destroyed Target" 1e+01)
          (else
            (Variables|Dissolve|SetTarget%20Dissolve 0.0)
            (Variables|Dissolve|SetDissolve%20Speed 4.0)
            (Utilities|Time|SetTimerbyFunctionName 0 "On Despawn" 1.0)
            (Collision|SetCollisionEnabled (Variables|Default|GetStaticMesh) "NoCollision"))))
      (:then_1
        (bind _asmain_gamemode (Utilities|Casting|CastToMainGamemode (Game|GetGameMode)))
        (bind _score_to_add (|GetScoreToAdd Focused Distance Heat Hits%20in%20a%20row (Variables|/Game/Main/Blueprints/Gamemode/MainGamemode.MainGamemode_C|GetTime%20Since%20Last%20Score _asmain_gamemode) (Variables|Default|GetSize) Hit%20By))
        (Default|AddPoints _asmain_gamemode _score_to_add)))))

(fn OnDespawn
  (Variables|Default|SetAvailable false)
  (Variables|Default|SetTargetable false)
  (Utilities|Time|SetTimerbyFunctionName 0 "On Cooldown Expired" 5.0))

(fn OnCooldownExpired
  (Variables|Default|SetAvailable true))

(fn HideDestroyedTarget
  (Development|SetHiddeninGame (Variables|Default|GetTarget_Collection) true false))